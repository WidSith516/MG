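; Spline path actor (xidePunk Easy Object Movement) that sets up configurable movement for a list of target objects.
; BeginPlay spawns and attaches a BP_Movement_Child per valid target, passing its speed, delay, loop, trigger and look-at settings.
; The construction script positions the spline, caches point indices and triggers, and runs debug markers, which also fill the look-at array.
; Helper functions switch curve or linear points, toggle looping and remove the last point.
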(event `self.ReceiveBeginPlay`
  ;[1 0 0 0.2] xidePunk - Easy Object Movement
  ;;[0 0 0] Send References to Movement Object
  (for _array_element (`self.Objects`)
    (bind (_targetobject _triggerobject _startmovementtype _beginplaydelay _overlapdelay _objectrotation _followrotationtosplinepoint _lookatrotation _loop _movementspeed _lookatspeed _destroywhenfinished _delay _delaytime) (break `/Game/EasyObjectMovement/Blueprint/F_ObjectMovement_Structure` _array_element))
    (`/Engine/EditorBlueprintResources/StandardMacros.IsValid` _targetobject
      (:`Is Valid`
        (bind _returnvalue (`KismetArrayLibrary.Array_Add` (`self.Target Object Array`) _targetobject))
        (for _ (range (+ _returnvalue 1))
          _)
        (bind _returnvalue_2 (`|SpawnActorFromClass` "/Game/EasyObjectMovement/Blueprint/Child/BP_Movement_Child.BP_Movement_Child_C" (`self.GetTransform`) "AlwaysSpawn" "OverrideRootScale" null (`self.Objects`) (`self.Target Object Array`) (`self.Trigger Object Array`) self _beginplaydelay _overlapdelay _destroywhenfinished _movementspeed (`self.Look At Rotation Array`) _startmovementtype _loop _followrotationtosplinepoint _lookatspeed _triggerobject _lookatrotation _delay _delaytime _objectrotation null))
        (`self.K2_AttachToActor` _returnvalue_2 self "None" "SnapToTarget" "SnapToTarget" "SnapToTarget" true)))))

(fn `Curve Spline`
  ;[0 0 0] Set Spline Curve
  (for _array_element (`self.Points`)
    (`SplineComponent.SetSplinePointType` (`self.Spline`) _array_element "Curve" true)))

(fn `Linear Spline`
  ;[0 0 0] Set Spline Linear
  (for _array_element (`self.Points`)
    (`SplineComponent.SetSplinePointType` (`self.Spline`) _array_element "Linear" true)))

(fn `Loop`
  ;[0 0 0] Set Loop to Spline
  (`SplineComponent.SetClosedLoop` (`self.Spline`) true true))

(fn `Not Loop`
  ;[0 0 0] Not Loop
  (`SplineComponent.SetClosedLoop` (`self.Spline`) false true))

(fn `Remove Last Point`
  (bind _returnvalue (`KismetArrayLibrary.Array_LastIndex` (`self.Points`)))
  ;[0 0 0] Remove Last Index in Spline
  (if (> _returnvalue 1)
    (`SplineComponent.RemoveSplinePoint` (`self.Spline`) _returnvalue true)
    (`KismetArrayLibrary.Array_Remove` (`self.Points`) _returnvalue)))

(fn `UserConstructionScript`
  (bind _look_at_rotation_array (`self.Look At Rotation Array`))
  (bind _spline (`self.Spline`))
  (bind _spline_origin_location (`self.Spline Origin Location`))
  ;[1 0 0 0.2] xidePunk - Easy Object Movement
  (`|ExecutionSequence`
    (:`then_0`
      ;;[0 0 0] Set Spline Origin
      (`/Engine/EditorBlueprintResources/StandardMacros.IsValid` _spline_origin_location
        (:`Is Valid`
          (`self.K2_SetActorLocation` (`self.K2_GetActorLocation` _spline_origin_location)))))
    (:`then_1`
      ;;[0 0 0] Spline Points
      (for _index (range -2 (+ (- (`SplineComponent.GetNumberOfSplinePoints` (`self.Spline`)) 2) 1))
        (`KismetArrayLibrary.Array_Add` (`self.Points`) (+ _index 1))))
    (:`then_2`
      ;;[0 0 0] Set Spline Pivot
      (`SceneComponent.K2_SetRelativeLocation` _spline (+ (`SceneComponent.RelativeLocation` _spline) (`self.Spline Pivot`)) false false))
    (:`then_3`
      (if (`self.Show Debug`)
        (`|ExecutionSequence`
          (:`then_0`
            (`|ExecutionSequence`
              (:`then_0`
                (for _array_element (`self.Objects`)
                  (`KismetArrayLibrary.Array_Add` _look_at_rotation_array (`.LookatRotation_25_A60ADDA246133167815944A9F461235A` (break `/Game/EasyObjectMovement/Blueprint/F_ObjectMovement_Structure` _array_element)))
                  (for _array_element_2 _look_at_rotation_array
                    (`/Engine/EditorBlueprintResources/StandardMacros.IsValid` _array_element_2
                      (:`Is Valid`
                        (bind _returnvalue (+ (`self.K2_GetActorLocation` _array_element_2) (0.0 0.0 177.0)))
                        (`AddComponent|NODE_AddBillboardComponent-2` :`bManualAttachment` true :`RelativeTransform` (`KismetMathLibrary.MakeTransform` _returnvalue (struct) (0.5 0.5 0.5)))
                        (`KismetSystemLibrary.DrawDebugLine` (`self.K2_GetActorLocation`) _returnvalue (struct :`R` 0.393713 :`B` 1.0 :`A` 1.0) 2.0 5.0))))))
              (:`then_1`
                (`SceneComponent.K2_SetWorldLocation` (`self.End`) (+ (`SplineComponent.GetLocationAtSplinePoint` (`self.Spline`) (`KismetArrayLibrary.Array_LastIndex` (`self.Points`)) "World") (0.0 0.0 177.0)) false false))))
          (:`then_1`
            (`SceneComponent.SetVisibility` (`self.Origin`) true false)
            (`SceneComponent.SetVisibility` (`self.End`) true false)))
        (else
          (`SceneComponent.SetVisibility` (`self.Origin`) false false)
          (`SceneComponent.SetVisibility` (`self.End`) false false))))
    (:`then_4`
      (for _array_element_3 (`self.Objects`)
        (bind ((`TriggerObject_4_BA752E394DE12C87063B3B8A06D24202` _triggerobject)) (break `/Game/EasyObjectMovement/Blueprint/F_ObjectMovement_Structure` _array_element_3))
        (`/Engine/EditorBlueprintResources/StandardMacros.IsValid` _triggerobject
          (:`Is Valid`
            (`KismetArrayLibrary.Array_Add` (`self.Trigger Object Array`) _triggerobject)))))))