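; BP_Resound is a pickup actor for a "resound", defined by musical note (音阶), timbre (音色) and quantity.
; The Construction Script builds a DT_Resounds row name from note and timbre, storing its index as the pickup component's ItemID, or -1 with debug prints if missing.
; It also selects the mesh by note and color material by timbre.
; Sphere1 overlaps call the component's IsPickUp, while Tick spins the mesh by random yaw steps.
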(event `self.Sphere1.OnComponentBeginOverlap`
  (params (OverlappedComponent :type "PrimitiveComponent Object Reference") (OtherActor :type "Actor Object Reference") (OtherComp :type "PrimitiveComponent Object Reference") (OtherBodyIndex :type Integer) (bFromSweep :type Boolean) (SweepResult :type "HitResult Structure (by ref)"))
  (`/Game/BTWY/PickUpItem/BPI_IsPickUp.IsPickUp` (`self.BPComp_IsPickUp`) OtherActor))

(event `self.ReceiveBeginPlay`)

(event `self.ReceiveTick`
  (params (DeltaSeconds :type "Float (single-precision)"))
  (bind _sphere (`self.Sphere`))
  (bind (_returnvalue_roll _returnvalue_pitch _returnvalue_yaw) (`KismetMathLibrary.BreakRotator` (`SceneComponent.K2_GetComponentRotation` _sphere)))
  (`SceneComponent.K2_SetWorldRotation` _sphere (`KismetMathLibrary.MakeRotator` _returnvalue_roll _returnvalue_pitch (+ _returnvalue_yaw (`KismetMathLibrary.RandomFloatInRange` 0.5 2.0))) false false))

(fn `UserConstructionScript`
  (bind _bpcomp_ispickup (`self.BPComp_IsPickUp`))
  (bind _returnvalue (`KismetStringLibrary.Concat_StrStr` (select `int` (`self.音色`) :`0` "" :`1` "yellow" :`2` "blue" :`3` "green" :`4` "red") "-" (`|GetEnumeratorNameAsString` (`self.音阶`)) (`KismetStringLibrary.Conv_IntToString` (`self.音色`))))
  (bind _returnvalue_2 (`KismetStringLibrary.Conv_StringToName` _returnvalue))
  (`|ExecutionSequence`
    (:`then_0`
      (set `/Game/BTWY/PickUpItem/BPComp_IsPickUp.Num` (`self.数量`) (`self.BPComp_IsPickUp`))
      (`|GetDataTableRow` "/Game/BTWY/Resounds/DT_Resounds.DT_Resounds" _returnvalue_2
        (:`then`
          (bind _outrownames (`DataTableFunctionLibrary.GetDataTableRowNames` "/Game/BTWY/Resounds/DT_Resounds.DT_Resounds"))
          (set `/Game/BTWY/PickUpItem/BPComp_IsPickUp.ItemID` (`KismetArrayLibrary.Array_Find` _outrownames _returnvalue_2) _bpcomp_ispickup))
        (:`RowNotFound`
          (`KismetSystemLibrary.PrintString` "没有找到此回响")
          (`KismetSystemLibrary.PrintString` _returnvalue)
          (set `/Game/BTWY/PickUpItem/BPComp_IsPickUp.ItemID` -1 _bpcomp_ispickup))))
    (:`then_1`
      (`StaticMeshComponent.SetStaticMesh` (`self.Sphere`) (select `/Game/BTWY/Resounds/E_MusicalScale` (`self.音阶`) :`NewEnumerator3` "/Game/BTWY/UI/Asset/拾取物/UI_UV修复版）__1__变.UI_UV修复版）__1__变" :`NewEnumerator1` "/Game/BTWY/UI/Asset/拾取物/UI_UV修复版）__1__商.UI_UV修复版）__1__商" :`NewEnumerator0` "/Game/BTWY/UI/Asset/拾取物/UI_UV修复版）__1__宫.UI_UV修复版）__1__宫" :`NewEnumerator4` "/Game/BTWY/UI/Asset/拾取物/UI_UV修复版）__1__徵.UI_UV修复版）__1__徵" :`NewEnumerator6` "/Game/BTWY/UI/Asset/拾取物/UI_UV修复版）__1__润.UI_UV修复版）__1__润" :`NewEnumerator5` "/Game/BTWY/UI/Asset/拾取物/UI_UV修复版）__1__羽.UI_UV修复版）__1__羽" :`NewEnumerator2` "/Game/BTWY/UI/Asset/拾取物/UI_UV修复版）__1__角.UI_UV修复版）__1__角" :!type "StaticMesh Object Reference"))
      (`PrimitiveComponent.SetMaterial` (`self.Sphere`) 0 (select `int` (`self.音色`) :`0` null :`1` "/Game/BTWY/UI/Asset/拾取物/UiYellow_Inst.UiYellow_Inst" :`2` "/Game/BTWY/UI/Asset/拾取物/UiBule_Inst.UiBule_Inst" :`3` "/Game/BTWY/UI/Asset/拾取物/UiGreen_Inst.UiGreen_Inst" :`4` "/Game/BTWY/UI/Asset/拾取物/UiRed_Inst.UiRed_Inst" :!type "MaterialInstance Object Reference")))))