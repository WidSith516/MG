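; Area background music trigger that plays an assigned MetaSound while the player is inside its box and layers it according to collected items.
; Tick runs through a Gate while inside, checking mapped backpack item IDs in the player's BPComp_PickUp.
; The first time each of six items is held, a shared timeline ramps the matching "Input" parameter.
; Leaving closes the Gate and fades volume out without stopping playback.
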(event `self.ReceiveBeginPlay`
  (`AudioComponent.Stop` (`self.MetaSound`))
  (set `self.Player` (`GameplayStatics.GetPlayerPawn` 0)))

(event `self.Box.OnComponentBeginOverlap`
  (params (OverlappedComponent :type "PrimitiveComponent Object Reference") (OtherActor :type "Actor Object Reference") (OtherComp :type "PrimitiveComponent Object Reference") (OtherBodyIndex :type Integer) (bFromSweep :type Boolean) (SweepResult :type "HitResult Structure (by ref)"))
  (if (== OtherActor (`GameplayStatics.GetPlayerPawn` 0))
    (`AudioComponent.SetVolumeMultiplier` (`self.MetaSound`) 1.0)
    (`AudioComponent.Play` (`self.MetaSound`) 0.0)
    (goto _label :!via `Open`)))

(event `self.ReceiveTick`
  (params (DeltaSeconds :type "Float (single-precision)"))
  (`/Engine/EditorBlueprintResources/StandardMacros.Gate` true :!label _label
    (:`Exit`
      (`/Engine/EditorBlueprintResources/StandardMacros.DoOnce` false :!label _label_2
        (:`Completed`
          (for (_array_element _array_index) (`self.metasound序号:背包ID`)
            (if (> (`/Game/BTWY/UI/Blueprint/背包/BP_BagItem.数量` (`|GetArrayItem` (`/Game/BTWY/PickUpItem/BPComp_PickUp.背包` (`self.GetComponentByClass` (`self.Player`) "/Game/BTWY/PickUpItem/BPComp_PickUp.BPComp_PickUp_C")) _array_element)) 0)
              (switch `int` _array_index
                (:`0`
                  (`/Engine/EditorBlueprintResources/StandardMacros.DoOnce` false
                    (:`Completed`
                      _)))
                (:`1`
                  (`/Engine/EditorBlueprintResources/StandardMacros.DoOnce` false
                    (:`Completed`
                      _)))
                (:`2`
                  (`/Engine/EditorBlueprintResources/StandardMacros.DoOnce` false
                    (:`Completed`
                      _)))
                (:`3`
                  (`/Engine/EditorBlueprintResources/StandardMacros.DoOnce` false
                    (:`Completed`
                      _)))
                (:`4`
                  (`/Engine/EditorBlueprintResources/StandardMacros.DoOnce` false
                    (:`Completed`
                      _)))
                (:`5`
                  (`/Engine/EditorBlueprintResources/StandardMacros.DoOnce` false
                    (:`Completed`
                      _))))
              (bind _output_get (set `self.Array Index` _array_index))
              (bind (_direction _float_0_1) (`Timeline|时间轴` :!via `PlayFromStart`)
                (:`Update`
                  (`AudioParameterControllerInterface.SetFloatParameter` (`self.MetaSound`) (`KismetStringLibrary.Conv_StringToName` (`KismetStringLibrary.Concat_StrStr` "Input" (`KismetStringLibrary.Conv_IntToString` _output_get))) _float_0_1)))))
          (goto _label_2 :!via `Reset`))))))

(event `self.Box.OnComponentEndOverlap`
  (params (OverlappedComponent :type "PrimitiveComponent Object Reference") (OtherActor :type "Actor Object Reference") (OtherComp :type "PrimitiveComponent Object Reference") (OtherBodyIndex :type Integer))
  (if (== OtherActor (`GameplayStatics.GetPlayerPawn` 0))
    (`|ExecutionSequence`
      (:`then_0`
        (goto _label :!via `Close`))
      (:`then_1`
        (bind (_direction _float_0_1) (`Timeline|时间轴_0` :!via `PlayFromStart`)
          (:`Update`
            (`AudioComponent.SetVolumeMultiplier` (`self.MetaSound`) (- 1.0 _float_0_1))))))))

(fn `UserConstructionScript`
  (`AudioComponent.SetSound` (`self.MetaSound`) (`self.BGM`)))