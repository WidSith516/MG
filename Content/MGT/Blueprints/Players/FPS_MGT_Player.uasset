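; First-person player Blueprint of the MGT character system, which blocks camera switching and keeps the weapon visible to other players.
; Every Tick, it removes HUD_Commands widgets and disables CanSwitchCam on the MGT player component.
; The local player's camera rotation replicates each frame through server and multicast events to remote copies.
; On non-local copies, the weapon attaches to Mesh2P at construction, then to Mesh's Gun_Socket every Tick.
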(event `self.ReceiveBeginPlay`
  (`parent.ReceiveBeginPlay`))

(event `self.ReceiveTick`
  (params (DeltaSeconds :type "Float (single-precision)"))
  (bind _bp_weapon_component (`self.BP_Weapon_Component`))
  (`parent.ReceiveTick` DeltaSeconds)
  (`self.PitchReplication`)
  ;[1 1 1] Forbid player to use the MGT Switch Cam system while using FPS class
  (bind _foundwidgets (`WidgetBlueprintLibrary.GetAllWidgetsOfClass` "/Game/MGT/Blueprints/HUD/HUD_Commands.HUD_Commands_C" false))
  (for _array_element _foundwidgets
    (`Widget.RemoveFromParent` _array_element))
  (set `/Game/MGT/Blueprints/Players/AC_MGT_PlayerComp.CanSwitchCam` false (`self.AC_MGT_PlayerComp`))
  ;[1 1 1] Attach the fun to third person that other players can see
  (if (not (`self.IsLocallyControlled`))
    (`SceneComponent.K2_AttachToComponent` _bp_weapon_component (`self.Mesh`) "Gun_Socket" "SnapToTarget" "SnapToTarget" "SnapToTarget" true)
    (`PrimitiveComponent.SetOnlyOwnerSee` _bp_weapon_component false)))

(event `PitchReplication`
  (if (`self.IsLocallyControlled`)
    (`self.S_PichReplication` (`SceneComponent.K2_GetComponentRotation` (`self.FollowCamera`)))))

(event `S_PichReplication`
  (params (CamPitch :type "Rotator Structure"))
  (bind _camrotation (`self.CamRotation`))
  (set `self.CamRotation` CamPitch)
  (`SceneComponent.K2_SetWorldRotation` (`self.FollowCamera`) _camrotation false false)
  (`self.M_PitchReplication` _camrotation))

(event `M_PitchReplication`
  (params (CamPitch :type "Rotator Structure"))
  (if (not (`self.IsLocallyControlled`))
    (`SceneComponent.K2_SetWorldRotation` (`self.FollowCamera`) CamPitch false false)))

(fn `OnRep_ControlRotation`)

(fn `UserConstructionScript`
  ;[0 1 0.8329] Attach gun to skeletal mesh - allow other player to see the bullet starting from where it should start
  (`parent.UserConstructionScript`)
  (if (not (`self.IsLocallyControlled`))
    (`SceneComponent.K2_AttachToComponent` (`self.BP_Weapon_Component`) (`self.Mesh2P`) "GripPoint" "SnapToTarget" "SnapToTarget" "SnapToTarget" true)))