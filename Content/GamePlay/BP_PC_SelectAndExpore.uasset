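; BP_PC_SelectAndExpore orients its actor relative to a spherical planet, using the direction away from PlanetCenter as up.
; Each Tick line-traces outward along that direction and stores the hit normal in GroundNormal, which feeds only an unused node.
; Only when the trace misses, it builds axes from the projected forward vector and sets rotation, interpolating from a location-derived rotation rather than the current one.
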(event `self.ReceiveTick`
  (params (DeltaSeconds :type "Float (single-precision)"))
  (bind _returnvalue (`self.K2_GetActorLocation`))
  (bind _returnvalue_2 (`KismetMathLibrary.NegateVector` (`KismetMathLibrary.Normal` (- (`self.PlanetCenter`) _returnvalue))))
  (bind (_outhit _returnvalue_3) (`KismetSystemLibrary.LineTraceSingle` _returnvalue (+ (* _returnvalue_2 (`self.TraceDistance`)) _returnvalue) "TraceTypeQuery1"))
  (if _returnvalue_3
    (bind _output_get (set `self.GroundNormal` (`.Normal` (`GameplayStatics.BreakHitResult` _outhit))))
    (else
      (bind _output_get_2 (set `self.DesiredUp` _returnvalue_2))
      (bind _output_get_3 (set `self.DesiredForward` (`KismetMathLibrary.Normal` (`KismetMathLibrary.ProjectVectorOnToPlane` (`self.GetActorForwardVector`) _output_get_2))))
      (bind _output_get_4 (set `self.DesiredRight` (`KismetMathLibrary.Normal` (`KismetMathLibrary.Cross_VectorVector` _output_get_3 _output_get_2))))
      (set `self.Rotator` (`KismetMathLibrary.MakeRotationFromAxes` (`self.DesiredForward`) _output_get_4 (`self.DesiredUp`)))
      (`self.K2_SetActorRotation` (`KismetMathLibrary.RInterpTo` (`KismetMathLibrary.Conv_VectorToRotator` (`self.K2_GetActorLocation`)) (`self.Rotator`) DeltaSeconds (`self.InterpSpeed`))))))

(fn `UserConstructionScript`)