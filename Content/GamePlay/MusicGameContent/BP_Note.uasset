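; BP_Note is a note actor for the music game that travels along its local X axis.
; Tick scales MovementSpeed by delta time and applies it as a local offset each frame.
; The HitBox overlap handler filters for other BP_Note actors and checks Judged, but ends in an empty branch, so it has no effect.
; An absolute timing-error calculation against NoteTime exists but is not connected.
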(event `self.ReceiveTick`
  (params (DeltaSeconds :type "Float (single-precision)"))
  (bind _result (`/Engine/EditorBlueprintResources/StandardMacros.NegateFloat` (* DeltaSeconds (`self.MovementSpeed`)))
    (:`  `
      (`self.K2_AddActorLocalOffset` (`KismetMathLibrary.MakeVector` _result)))))

(event `self.HitBox.OnComponentBeginOverlap`
  (params (OverlappedComponent :type "PrimitiveComponent Object Reference") (OtherActor :type "Actor Object Reference") (OtherComp :type "PrimitiveComponent Object Reference") (OtherBodyIndex :type Integer) (bFromSweep :type Boolean) (SweepResult :type "HitResult Structure (by ref)"))
  (cast `/Game/GamePlay/MusicGameContent/BP_Note` OtherActor)
  (if (`self.bJudged`)
    _
    (elif true
      _)))

(fn `UserConstructionScript`)