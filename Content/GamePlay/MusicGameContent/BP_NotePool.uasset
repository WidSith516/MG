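; BP_NotePool is a music-game note spawner that plays a sound at BeginPlay and spawns BP_Note actors from DT_LevelMusicData_1.
; It records the music start time, then loops once through the table rows, spawning notes whose StartTime minus TimeOffset has already elapsed.
; Later notes are never rechecked, as Tick is empty.
; Despite the name there is no pooling: NextFreeIndex is unused and each spawned note gets a zero NoteTime.
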(event `self.ReceiveBeginPlay`
  (set `self.MusicStartTime` (`KismetSystemLibrary.GetGameTimeInSeconds`))
  (`GameplayStatics.PlaySound2D` null 1.0 1.0 0.0 null null)
  (bind _outrownames (`DataTableFunctionLibrary.GetDataTableRowNames` "/Game/GamePlay/DT_LevelMusicData_1.DT_LevelMusicData_1"))
  (for _array_element _outrownames
    (bind _returnvalue (`|GetDataTableRow` "/Game/GamePlay/DT_LevelMusicData_1.DT_LevelMusicData_1" _array_element)
      (:`then`
        (if (>= (- (`KismetSystemLibrary.GetGameTimeInSeconds`) (`self.MusicStartTime`)) (- (`.StartTime_8_CA4D3A75478C09555AD1E083C90E570E` (break `/Game/GamePlay/EStruct_NoteData` _returnvalue)) (`self.TimeOffset`)))
          (bind _returnvalue_2 (`|SpawnActorFromClass` "/Game/GamePlay/MusicGameContent/BP_Note.BP_Note_C" (struct) "AdjustIfPossibleButDontSpawnIfColliding" "MultiplyWithRoot" null null))
          (set `/Game/GamePlay/MusicGameContent/BP_Note.NoteTime` 0.0 _returnvalue_2))))))

(fn `UserConstructionScript`)