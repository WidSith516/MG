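; BP_Ending_Lost is an actor that sets up the losing ending screen when play begins.
; It loops over every CameraActor in the level, blending the player view to each and creating an Ending_Lost widget each time.
; Each pass also locks input to that UI and enables the mouse cursor, click and hover events, then prints an initialization-complete message.
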(event `self.ReceiveBeginPlay`
  (bind _pc (`self.PC`))
  (bind _output_get (set `self.PC` (`GameplayStatics.GetPlayerController` 0)))
  (bind _outactors (`GameplayStatics.GetAllActorsOfClass` "/Script/Engine.CameraActor"))
  (for _array_element _outactors
    (set `self.EndingCameraRef` _array_element)
    (`PlayerController.SetViewTargetWithBlend` _output_get (`self.EndingCameraRef`) 1.5 "VTBlend_Linear" 0.0 false)
    (bind _returnvalue (`|CreateWidget` "/Game/GamePlay/WBP/Ending_Lost.Ending_Lost_C" (`self.PC`)))
    (set `self.EndingUI` _returnvalue)
    (`UserWidget.AddToViewport` (`self.EndingUI`) 0)
    (`WidgetBlueprintLibrary.SetInputMode_UIOnlyEx` (`self.PC`) (`self.EndingUI`) "LockAlways")
    (set `PlayerController.bShowMouseCursor` true _pc)
    (set `PlayerController.bEnableClickEvents` true _pc)
    (set `PlayerController.bEnableMouseOverEvents` true _pc)
    (`KismetSystemLibrary.PrintString` "结局初始化完毕")))

(fn `UserConstructionScript`)