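; Game mode that holds the level's audio and scaffolds an unfinished audio analysis pass.
; BeginPlay queries cooked FFT data without using it, binds an empty playback-percent handler and flags audio as playing; audio finishing clears the flag.
; SoundAnalyzer, never called, would busy-loop without a delay, updating elapsed time while that flag is set.
; Constant-Q analyzer lookups per channel are left disconnected.
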(event `self.ReceiveBeginPlay`
  (`AudioComponent.GetCookedFFTDataForAllPlayingSounds` (`self.LevelAudio`))
  (add `AudioComponent.OnAudioPlaybackPercent` (`self.LevelAudio`) (delegate `OnAudioPlaybackPercent_事件`))
  (set `self.isAudioPlaying` true))

(event `OnAudioPlaybackPercent_事件`
  (params (PlayingSoundWave :type "SoundWave Object Reference") (PlaybackPercent :type "Float (single-precision)")))

(event `self.ReceiveTick`
  (params (DeltaSeconds :type "Float (single-precision)")))

(event `self.LevelAudio.OnAudioFinished`
  (set `self.isAudioPlaying` false))

(fn `SoundAnalyzer`
  (set `self.StartTime` (`KismetSystemLibrary.GetGameTimeInSeconds`))
  (while (`self.isAudioPlaying`)
    (`self.UpdateCurrentTime`))
  (`KismetSystemLibrary.PrintText` "AudioPlayFinished"))

(fn `UpdateCurrentTime`
  (set `self.CurrentTime` (- (`KismetSystemLibrary.GetGameTimeInSeconds`) (`self.StartTime`))))

(fn `UserConstructionScript`)