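; BP_L2_PlayerController is a player controller that turns input into one-shot percussion and sample sounds.
; On BeginPlay it adds the IMC_MG_gameplay Enhanced Input mapping context.
; Seven input actions, named for keys Z through M, each play their own 2D sound cue.
; CheckCollisionByIndex is an unfinished stub that only gathers actors and is never called here.
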(event `self.ReceiveBeginPlay`
  (`EnhancedInputSubsystemInterface.AddMappingContext` (pcsubsystem `EnhancedInputLocalPlayerSubsystem` null) "/Game/GamePlay/Sounds/IMC_MG_gameplay.IMC_MG_gameplay" 0 (struct)))

(event `EnhancedInput|/Game/GamePlay/Sounds/IA_1Z`
  (params (ActionValue :type Boolean) (ElapsedSeconds :type "Float (double-precision)") (TriggeredSeconds :type "Float (double-precision)") (InputAction :type "InputAction Object Reference" :default "/Game/GamePlay/Sounds/IA_1Z.IA_1Z"))
  (:`Triggered`
    (`GameplayStatics.PlaySound2D` "/Game/LevelMusic/SE/28/Group3_Beat/Z-3-bassdrop_Cue.Z-3-bassdrop_Cue" 1.0 1.0 0.0 null null)))

(event `EnhancedInput|/Game/GamePlay/Sounds/IA_2X`
  (params (ActionValue :type Boolean) (ElapsedSeconds :type "Float (double-precision)") (TriggeredSeconds :type "Float (double-precision)") (InputAction :type "InputAction Object Reference" :default "/Game/GamePlay/Sounds/IA_2X.IA_2X"))
  (:`Triggered`
    (`GameplayStatics.PlaySound2D` "/Game/LevelMusic/SE/28/Group3_Beat/X-3-samplemetal2_Cue.X-3-samplemetal2_Cue" 1.0 1.0 0.0 null null)))

(event `EnhancedInput|/Game/GamePlay/Sounds/IA_3C`
  (params (ActionValue :type Boolean) (ElapsedSeconds :type "Float (double-precision)") (TriggeredSeconds :type "Float (double-precision)") (InputAction :type "InputAction Object Reference" :default "/Game/GamePlay/Sounds/IA_3C.IA_3C"))
  (:`Triggered`
    (`GameplayStatics.PlaySound2D` "/Game/LevelMusic/SE/28/Group3_Beat/C-3-kick_Cue.C-3-kick_Cue" 1.0 1.0 0.0 null null)))

(event `EnhancedInput|/Game/GamePlay/Sounds/IA_4V`
  (params (ActionValue :type Boolean) (ElapsedSeconds :type "Float (double-precision)") (TriggeredSeconds :type "Float (double-precision)") (InputAction :type "InputAction Object Reference" :default "/Game/GamePlay/Sounds/IA_4V.IA_4V"))
  (:`Triggered`
    (`GameplayStatics.PlaySound2D` "/Game/LevelMusic/SE/28/Group3_Beat/V-3-pop_Cue.V-3-pop_Cue" 1.0 1.0 0.0 null null)))

(event `EnhancedInput|/Game/GamePlay/Sounds/IA_5B`
  (params (ActionValue :type Boolean) (ElapsedSeconds :type "Float (double-precision)") (TriggeredSeconds :type "Float (double-precision)") (InputAction :type "InputAction Object Reference" :default "/Game/GamePlay/Sounds/IA_5B.IA_5B"))
  (:`Triggered`
    (`GameplayStatics.PlaySound2D` "/Game/LevelMusic/SE/28/Group3_Beat/B-3-samplmetal1_Cue.B-3-samplmetal1_Cue" 1.0 1.0 0.0 null null)))

(event `EnhancedInput|/Game/GamePlay/Sounds/IA_6N`
  (params (ActionValue :type Boolean) (ElapsedSeconds :type "Float (double-precision)") (TriggeredSeconds :type "Float (double-precision)") (InputAction :type "InputAction Object Reference" :default "/Game/GamePlay/Sounds/IA_6N.IA_6N"))
  (:`Triggered`
    (`GameplayStatics.PlaySound2D` "/Game/LevelMusic/SE/28/Group3_Beat/N-3-waterdrum_Cue.N-3-waterdrum_Cue" 1.0 1.0 0.0 null null)))

(event `EnhancedInput|/Game/GamePlay/Sounds/IA_7M`
  (params (ActionValue :type Boolean) (ElapsedSeconds :type "Float (double-precision)") (TriggeredSeconds :type "Float (double-precision)") (InputAction :type "InputAction Object Reference" :default "/Game/GamePlay/Sounds/IA_7M.IA_7M"))
  (:`Triggered`
    (`GameplayStatics.PlaySound2D` "/Game/LevelMusic/SE/28/Group3_Beat/M-3-pulsation_Cue.M-3-pulsation_Cue" 1.0 1.0 0.0 null null)))

(fn `CheckCollisionByIndex`
  (`GameplayStatics.GetAllActorsOfClass` null))

(fn `UserConstructionScript`)